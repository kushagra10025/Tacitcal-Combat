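; Grid actor that builds a tile grid of squares, hexagons or triangles as mesh instances from its construction script.
; SpawnGrid clears old instances, pulls the shape's mesh and border material from DT_GridShapeData, then snaps the center and derives the bottom-left corner.
; Each index maps to a transform through per-shape spacing.
; Hexagons use doubled-row indices, stepping Y by two with alternating starts, and triangles flip yaw by index parity.
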(fn `CalculateCenterAndBottomLeft`
  (returns (Center :type "Vector Structure") (BottomLeft :type "Vector Structure"))
  (locals (LCenterOfGrid :type "Vector Structure" :default (0.0 0.0 0.0)))
  (bind (_gridtilecount_x _gridtilecount_y) (`KismetMathLibrary.BreakVector2D` (`self.GridTileCount`)))
  (switch `/Game/Blueprints/Core/Grid/GridShapes/E_GridShape` (`self.GridShape`)
    (:`NewEnumerator0`
      ;[1 0 0.4922] For Square
      ;;[1 0.8438 0] Center Calculation
      (set `local.LCenterOfGrid` (`/Game/Blueprints/Core/Utils/BFL_Utilities.SnapVectorToVector` (`self.GridCenterLocation`) (`self.GridTileSize`)))
      (return (`local.LCenterOfGrid`) (- (`local.LCenterOfGrid`) (* (`self.DIV_Vec2_by_Float` (- (`self.GridTileCount`) (`KismetMathLibrary.MakeVector2D` (`KismetMathLibrary.SelectFloat` 0.0 1.0 (`/Game/Blueprints/Core/Utils/BFL_Utilities.IsFloatEven?` _gridtilecount_x)) (`KismetMathLibrary.SelectFloat` 0.0 1.0 (`/Game/Blueprints/Core/Utils/BFL_Utilities.IsFloatEven?` _gridtilecount_y)))) 2.0) (`KismetMathLibrary.Conv_VectorToVector2D` (`self.GridTileSize`))))))
    (:`NewEnumerator1`
      ;[1 0 0.4922] For Hexagon
      ;;[1 0.8438 0] Center Calculation
      (set `local.LCenterOfGrid` (`/Game/Blueprints/Core/Utils/BFL_Utilities.SnapVectorToVector` (`self.GridCenterLocation`) (* (`self.GridTileSize`) (1.5 1.0 1.0))))
      (return (`local.LCenterOfGrid`) (- (`local.LCenterOfGrid`) (`/Game/Blueprints/Core/Utils/BFL_Utilities.SnapVectorToVector` (* (/ (`self.GridTileCount`) (3.0 2.0)) (`KismetMathLibrary.Conv_VectorToVector2D` (`self.GridTileSize`))) (* (`self.GridTileSize`) (1.5 1.0 1.0))))))
    (:`NewEnumerator2`
      ;[1 0 0.4922] For Triangle
      ;;[1 0.8438 0] Center Calculation
      (set `local.LCenterOfGrid` (`/Game/Blueprints/Core/Utils/BFL_Utilities.SnapVectorToVector` (`self.GridCenterLocation`) (* (`self.GridTileSize`) (2.0 1.0 1.0))))
      (return (`local.LCenterOfGrid`) (- (`local.LCenterOfGrid`) (`/Game/Blueprints/Core/Utils/BFL_Utilities.SnapVectorToVector` (* (/ (- (`self.GridTileCount`) (0.0 0.0)) (2.0 4.0)) (`KismetMathLibrary.Conv_VectorToVector2D` (`self.GridTileSize`))) (* (`self.GridTileSize`) (2.0 1.0 1.0))))))))

(fn `DestroyGrid`
  (`InstancedStaticMeshComponent.ClearInstances` (`self.InstancedStaticMesh`))
  (return))

(fn `GetCurrentShapeData`
  (returns (ReturnValue :type "/Game/Blueprints/Core/Grid/GridShapes/S_GridShapeData Structure"))
  (bind _returnvalue (`|GetEnumeratorNameAsString` (`self.GridShape`)))
  (bind _returnvalue_2 (`|GetDataTableRow` "/Game/Blueprints/Core/Grid/GridShapes/DT_GridShapeData.DT_GridShapeData" (`KismetStringLibrary.Conv_StringToName` _returnvalue))
    (:`then`
      (return _returnvalue_2))
    (:`RowNotFound`
      (`KismetSystemLibrary.PrintString` (`KismetStringLibrary.Concat_StrStr` "Error - Row Not Found" _returnvalue) true true (struct :`R` 1.0 :`G` 0.106791 :`A` 1.0) 5.0)
      (return))))

(fn `GetTileLocationFromGridIndex`
  (params (GridIndex :type "Vector2D Structure"))
  (returns (TileLocation :type "Vector Structure"))
  (return (+ (`self.GridBottomLeftCornerLocation`) (* (`self.GridTileSize`) (`KismetMathLibrary.Conv_Vector2DToVector` (* (`local.GridIndex`) (select `/Game/Blueprints/Core/Grid/GridShapes/E_GridShape` (`self.GridShape`) :`NewEnumerator3` (1.0 1.0) :`NewEnumerator0` (1.0 1.0) :`NewEnumerator1` (0.75 0.5) :`NewEnumerator2` (1.0 0.5) :!type "Vector2D Structure")))))))

(fn `GetTileRotationFromGridIndex`
  (params (GridIndex :type "Vector2D Structure"))
  (returns (TileRotation :type "Rotator Structure"))
  (bind (_gridindex_x _gridindex_y) (`KismetMathLibrary.BreakVector2D` (`local.GridIndex`)))
  (if (`|EnumEquality` (`self.GridShape`) "NewEnumerator2")
    (return (`KismetMathLibrary.MakeRotator` 0.0 0.0 (+ (`KismetMathLibrary.SelectFloat` 180.0 0.0 (`/Game/Blueprints/Core/Utils/BFL_Utilities.IsFloatEven?` _gridindex_x)) (`KismetMathLibrary.SelectFloat` 180.0 0.0 (`/Game/Blueprints/Core/Utils/BFL_Utilities.IsFloatEven?` _gridindex_y)))))
    (else
      (return))))

(fn `SpawnGrid`
  (params (CenterLocation :type "Vector Structure") (TileSize :type "Vector Structure") (TileCount :type "Vector2D Structure") (Shape :type "/Game/Blueprints/Core/Grid/GridShapes/E_GridShape Enum" :default "NewEnumerator3"))
  (locals (LocalX :type Integer) (LocalY :type Integer) (LTileTransform :type "Transform Structure") (LIndex :type "Vector2D Structure"))
  (bind _instancedstaticmesh (`self.InstancedStaticMesh`))
  (bind _gridtilecount_x (`KismetMathLibrary.BreakVector2D` (`self.GridTileCount`)))
  (bind (_tilecount_x _tilecount_y) (`KismetMathLibrary.BreakVector2D` (`local.TileCount`)))
  (bind _lindex (`local.LIndex`))
  (bind (_gridtilecount_x_2 _gridtilecount_y) (`KismetMathLibrary.BreakVector2D` (`self.GridTileCount`)))
  (bind (_gridtilecount_x_3 _gridtilecount_y_2) (`KismetMathLibrary.BreakVector2D` (`self.GridTileCount`)))
  (bind ((`FlatMesh_12_5C2E8A4C4AD40686159749A18FF456A4` _flatmesh) (`FlatBorderMaterial_15_255F5B6941ED82FDA771D7BA68F0B37C` _flatbordermaterial)) (break `/Game/Blueprints/Core/Grid/GridShapes/S_GridShapeData` (`self.GetCurrentShapeData`)))
  ;[0 0.7891 1] Initialize Variables
  (set `self.GridCenterLocation` CenterLocation)
  (set `self.GridTileSize` TileSize)
  (set `self.GridShape` Shape)
  (set `self.GridTileCount` (`KismetMathLibrary.MakeVector2D` (`KismetMathLibrary.Conv_IntToDouble` (`KismetMathLibrary.Round` _tilecount_x)) (`KismetMathLibrary.Conv_IntToDouble` (`KismetMathLibrary.Round` _tilecount_y))))
  (`self.DestroyGrid`)
  ;[0.5234 0 1] Change Grid Mesh based on Input
  (`StaticMeshComponent.SetStaticMesh` _instancedstaticmesh _flatmesh)
  (`PrimitiveComponent.SetMaterial` _instancedstaticmesh 0 _flatbordermaterial)
  ;[1 0.375 0] Calculate Grid Center & Bottom Left Corner Location
  (bind (_center _bottomleft) (`self.CalculateCenterAndBottomLeft`))
  (set `self.GridCenterLocation` _center)
  (set `self.GridBottomLeftCornerLocation` _bottomleft)
  ;[1 0 0.04687] For Loop X & Y, for creating instances from bottom corner at X & Y Positions
  (for _index (range (`KismetMathLibrary.Round` _gridtilecount_x))
    (set `local.LocalX` _index)
    ;;[0 0.9062 1] Process Index Based on Hexagon or Not
    (if (`|EnumInequality` (`self.GridShape`) "NewEnumerator1")
      ;;[0 1 0.9766] If not Hexagon Index is Processed like this
      (for _index_2 (range (`KismetMathLibrary.Round` _gridtilecount_y))
        (set `local.LocalY` _index_2)
        ;[0.9688 0 1] Update Index
        (set `local.LIndex` (`KismetMathLibrary.MakeVector2D` (`KismetMathLibrary.Conv_IntToDouble` (`local.LocalX`)) (`KismetMathLibrary.Conv_IntToDouble` (`local.LocalY`))) :!label _label)
        ;[1 0.7031 0] Find the Tile transform based on Index and Bottom Corner Variables and Set Transform for Instanced Mesh
        (bind _output_get (set `local.LTileTransform` (`KismetMathLibrary.MakeTransform` (`self.GetTileLocationFromGridIndex` _lindex) (`self.GetTileRotationFromGridIndex` _lindex) (/ (`self.GridTileSize`) (`.MeshSize_3_8B736C434AB760D7F14016AA2C771501` (break `/Game/Blueprints/Core/Grid/GridShapes/S_GridShapeData` (`self.GetCurrentShapeData`)))))))
        (`InstancedStaticMeshComponent.AddInstance` (`self.InstancedStaticMesh`) _output_get true))
      (else
        ;;[0 1 0.8125] If Hexagon Index is Processed Like This
        (for _index_3 (range (`KismetMathLibrary.SelectInt` 0 1 (`/Game/Blueprints/Core/Utils/BFL_Utilities.IsIntegerEven?` (`local.LocalX`))) (* (`KismetMathLibrary.Round` _gridtilecount_y_2) 2))
          (set `local.LocalY` _index_3)
          (`|ExecutionSequence`
            (:`then_0`
              (goto _label))
            (:`then_1`
              (`/Engine/EditorBlueprintResources/StandardMacros.IncrementInt` _index_3))))))))

(fn `UserConstructionScript`
  (`self.SpawnGrid` (`self.K2_GetActorLocation`) (`self.GridTileSize`) (`self.GridTileCount`) (`self.GridShape`)))