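; BP_GridVisual is the visual layer of a grid, drawing its walkable tiles as instanced meshes.
; On initialization it takes the flat mesh and border material from the grid's current shape data, passes them to a child BP_GridMeshInst with query-only collision, and centers itself at the world origin with a Z offset from the ground.
; Tile updates remove the indexed instance and re-add it only if walkable; destroying clears all instances.
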(fn `DestroyGridVisual`
  (bind _gridmeshinstref (`self.GridMeshInstRef`)
    (:`then`
      (`/Game/Blueprints/Core/Grid/Utilities/BP_GridMeshInst.ClearInstances` _gridmeshinstref))
    (:`else`)))

(fn `InitializeGridVisual`
  (params (Grid :type "/Game/Blueprints/Core/Grid/BP_Grid Object Reference"))
  (bind ((`FlatMesh_12_5C2E8A4C4AD40686159749A18FF456A4` _flatmesh) (`FlatBorderMaterial_15_255F5B6941ED82FDA771D7BA68F0B37C` _flatbordermaterial)) (break `/Game/Blueprints/Core/Grid/GridShapes/S_GridShapeData` (`/Game/Blueprints/Core/Grid/BP_Grid.GetCurrentShapeData` (`self.GridRef`))))
  (set `self.GridRef` Grid)
  (set `self.GridMeshInstRef` (cast `/Game/Blueprints/Core/Grid/Utilities/BP_GridMeshInst` (`ChildActorComponent.ChildActor` (`self.ChildActor_GridMeshInst`)) :!pure true))
  (`/Game/Blueprints/Core/Grid/Utilities/BP_GridMeshInst.InitializeGridMeshInst` :`self` (`self.GridMeshInstRef`) :`Mesh` _flatmesh :`Material` _flatbordermaterial :`Collision` "QueryOnly")
  (`self.K2_SetActorLocation` (0.0 0.0 0.0)) ; Center Grid In World
  (`self.SetOffsetFromGround` (`self.ZOffset`)))

(fn `SetOffsetFromGround`
  (params (ZOffset :type "Float (double-precision)"))
  (bind (_returnvalue_x _returnvalue_y) (`KismetMathLibrary.BreakVector` (`self.K2_GetActorLocation`)))
  (set `self.ZOffset` ZOffset)
  (`self.K2_SetActorLocation` (`KismetMathLibrary.MakeVector` _returnvalue_x _returnvalue_y (`self.ZOffset`))))

(fn `UpdateTileVisual`
  (params (Data :type "/Game/Blueprints/Core/Grid/Utilities/S_TileData Structure"))
  (bind (_data_index _data_type _data_transform) (break `/Game/Blueprints/Core/Grid/Utilities/S_TileData` (`local.Data`)))
  (bind (_data_index_2 _data_type_2) (break `/Game/Blueprints/Core/Grid/Utilities/S_TileData` (`local.Data`)))
  (`/Game/Blueprints/Core/Grid/Utilities/BP_GridMeshInst.RemoveInstance` (`self.GridMeshInstRef`) _data_index_2)
  (if (`/Game/Blueprints/Core/Grid/Utilities/BFL_TileData.IsTileTypeWalkable` _data_type_2)
    (`/Game/Blueprints/Core/Grid/Utilities/BP_GridMeshInst.AddInstance` (`self.GridMeshInstRef`) _data_transform false _data_index)))

(fn `UserConstructionScript`)