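; Level loading Blueprint that keeps track of one active streaming sublevel and swaps it for another by name.
; On BeginPlay it force-loads the level named in LevelLoaded.
; LoadLevel skips repeat requests unless forced, hides and unloads the current level, then stores, loads and shows the new one.
; It prints an error when the new name matches no streaming level, except for "None".
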(event `self.ReceiveBeginPlay`
  (`self.LoadLevel` (`self.LevelLoaded`) true))

(fn `LoadLevel`
  (params (LevelName :type String) (bForceLoadLevel :type Boolean))
  (bind _returnvalue (`GameplayStatics.GetStreamingLevel` (`KismetStringLibrary.Conv_StringToName` (`self.LevelLoaded`))))
  (if (or (`KismetStringLibrary.NotEqual_StrStr` (`local.LevelName`) (`self.LevelLoaded`)) (`local.bForceLoadLevel`))
    (`|ExecutionSequence`
      (:`then_0`
        ;[1 0 0.8906] Unload the Currently Loaded Level
        (`/Engine/EditorBlueprintResources/StandardMacros.IsValid` _returnvalue
          (:`Is Valid`
            (set `LevelStreaming.bShouldBeVisible` false _returnvalue)
            (set `LevelStreaming.bShouldBeLoaded` false _returnvalue))))
      (:`then_1`
        ;[0.6641 1 0] Load the Passed Level and Save it to be unloaded Further
        (bind _output_get (set `self.LevelLoaded` (`local.LevelName`)))
        (bind _returnvalue_2 (`GameplayStatics.GetStreamingLevel` (`KismetStringLibrary.Conv_StringToName` _output_get)))
        (`/Engine/EditorBlueprintResources/StandardMacros.IsValid` _returnvalue_2
          (:`Is Valid`
            (set `LevelStreaming.bShouldBeLoaded` true _returnvalue_2)
            (set `LevelStreaming.bShouldBeVisible` true _returnvalue_2))
          (:`Is Not Valid`
            (if (`KismetStringLibrary.NotEqual_StrStr` (`self.LevelLoaded`))
              (`KismetSystemLibrary.PrintString` (`KismetStringLibrary.Concat_StrStr` "Error - LoadLevel - Invalid Level Name:" (`self.LevelLoaded`))))))))
    (else
      (return))))

(fn `UserConstructionScript`)